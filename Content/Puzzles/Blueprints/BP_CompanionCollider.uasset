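; BP_CompanionCollider is a trigger box that ends the game in a win when both companions are free.
; On overlap it checks the Companion, FirstSetFree and SecondSetFree variables, without testing which actor overlapped.
; It then disables player input, spawns particles at the player and plays a victory montage and sound.
; After a short delay it shows the GameWonMenu widget, pauses the game and reveals the cursor.
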(event OnComponentBeginOverlap(Box)
  (params (OverlappedComponent :type Primitive%20Component%20Object%20Reference) (OtherActor :type Actor%20Object%20Reference) (OtherComp :type Primitive%20Component%20Object%20Reference) (OtherBodyIndex :type Integer) (bFromSweep :type Boolean) (SweepResult :type Hit%20Result%20Structure%20%28by%20ref%29))
  (bind _returnvalue (Game|GetPlayerCharacter 0))
  (bind _returnvalue_2 (Transformation|GetActorLocation _returnvalue))
  ;[0.04971 0.04971 0.04971] If both companions are free then display game won menu
  (if (Variables|Default|GetCompanion)
    (if (Variables|Default|GetFirstSetFree)
      (if (Variables|Default|GetSecondSetFree)
        (bind _asbp_player_character (Utilities|Casting|CastToBP_PlayerCharacter _returnvalue))
        (Input|DisableInput _asbp_player_character (Game|GetPlayerController 0))
        (Effects|SpawnEmitteratLocation "/Game/VisualEffects/RealisticVFX/Particles/Sparks/P_Sparks_B.P_Sparks_B" _returnvalue_2 "0, 0, 0" "1.000000,1.000000,1.000000" false)
        (Effects|SpawnEmitteratLocation "/Game/VisualEffects/RealisticVFX/Particles/Environment/P_Butterfly.P_Butterfly" _returnvalue_2)
        (Animation|PlayAnimMontage _asbp_player_character "/Game/ThirdPerson/Animations/VictoryMontage.VictoryMontage" 1.0 "None")
        (Audio|PlaySound2D "/Game/SoundsEffects/InterfaceAndItemSounds/WAV/Special_Powerup_06.Special_Powerup_06" 1.0 1.0 0.0 0 0)
        (Utilities|FlowControl|Delay 3.5)
        (bind _returnvalue_3 (UserInterface|CreateWidget "/Game/UI/Menus/GameWonMenu.GameWonMenu_C"))
        (UserInterface|Viewport|AddtoViewport _returnvalue_3 0)
        (Game|SetGamePaused true)
        (Variables|/Script/Engine.PlayerController|SetbShowMouseCursor (Game|GetPlayerController 0) true)))))

(fn ConstructionScript)