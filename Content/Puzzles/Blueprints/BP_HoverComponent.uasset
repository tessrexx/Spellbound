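; BP_HoverComponent is a scene component that makes its owning actor hover above surfaces using physics.
; On BeginPlay it enables physics simulation on the owner's first primitive component.
; Each tick it traces downward and, on a hit, pushes that primitive along the surface normal with a force that fades linearly to zero at the trace length.
; A hit also applies the configured linear and angular damping, which is not reset when the trace misses.
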(event EventBeginPlay
  (bind _output_get (Variables|Default|Setvar_PrimitiveComponent (Utilities|Array|Get(acopy) (Actor|GetComponentsByClass (Components|GetOwner) "/Script/Engine.PrimitiveComponent"))))
  (Physics|SetSimulatePhysics _output_get true))

(event EventTick
  (params (DeltaSeconds :type Float%20%28single-precision%29))
  (bind _returnvalue (Transformation|GetWorldLocation))
  (bind (_outhit _returnvalue_2) (Collision|LineTraceByChannel _returnvalue (- _returnvalue (Math|Vector|MakeVector 0.0 0.0 (Variables|Default|Getvar_TraceLength))) "TraceTypeQuery1" true 0 "None"))
  (if _returnvalue_2
    (Physics|AddForce (Variables|Default|Getvar_PrimitiveComponent) (* (.ImpactNormal (Collision|BreakHitResult _outhit)) (Math|Float|Lerp (Variables|Default|Getvar_HoverForce) 0.0 (/ (Math|Vector|VectorLength (- (.Location (Collision|BreakHitResult _outhit)) (Transformation|GetWorldLocation))) (Variables|Default|Getvar_TraceLength)))) "None" false)
    (Class|PrimitiveComponent|SetLinearDamping (Variables|Default|Getvar_PrimitiveComponent) (Variables|Default|Getvar_LinearDamping))
    (Class|PrimitiveComponent|SetAngularDamping (Variables|Default|Getvar_PrimitiveComponent) (Variables|Default|Getvar_AngularDamping))))