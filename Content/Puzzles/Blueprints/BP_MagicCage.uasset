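; BP_MagicCage is a puzzle cage that traps companions until target spells break it.
; Each spell overlap lowers Structure and shrinks Fx2; at zero, per the comments the fifth hit, it bursts with lightning, then is destroyed with a butterfly effect.
; Box overlap sets the companion's IsTrapped flag for a dizzy animation.
; End overlap clears it, plays a falling montage and sound, and calls FollowPlayer.
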(event OnComponentBeginOverlap(Box)
  (params (OverlappedComponent :type Primitive%20Component%20Object%20Reference) (OtherActor :type Actor%20Object%20Reference) (OtherComp :type Primitive%20Component%20Object%20Reference) (OtherBodyIndex :type Integer) (bFromSweep :type Boolean) (SweepResult :type Hit%20Result%20Structure%20%28by%20ref%29))
  ;[0.04971 0.04971 0.04971] Sets Companion to IsTrapped to trigger dizzy anim in AnimBP
  (bind _asbp_parent_companion (Utilities|Casting|CastToBP_ParentCompanion OtherActor))
  (Variables|/Game/ThirdPerson/Blueprints/BP_ParentCompanion.BP_ParentCompanion_C|SetIsTrapped? _asbp_parent_companion true))

(event OnComponentEndOverlap(Box)
  (params (OverlappedComponent :type Primitive%20Component%20Object%20Reference) (OtherActor :type Actor%20Object%20Reference) (OtherComp :type Primitive%20Component%20Object%20Reference) (OtherBodyIndex :type Integer))
  ;[0.04971 0.04971 0.04971] Sets Companion to not trapped and triggers Follow Player Event
  (bind _asbp_parent_companion (Utilities|Casting|CastToBP_ParentCompanion OtherActor))
  (Animation|PlayAnimMontage _asbp_parent_companion "/Game/ThirdPerson/Animations/FallingMontage.FallingMontage" 1.0 "None")
  (Audio|PlaySoundatLocation "/Game/SoundsEffects/InterfaceAndItemSounds/WAV/Cartoon_Falling_04.Cartoon_Falling_04" (Transformation|GetActorLocation _asbp_parent_companion) "0, 0, 0" 1.0 1.0 0.0 0 0 0 0)
  (Variables|/Game/ThirdPerson/Blueprints/BP_ParentCompanion.BP_ParentCompanion_C|SetIsTrapped? _asbp_parent_companion false)
  (Default|FollowPlayer _asbp_parent_companion))

(event Collision|EventActorBeginOverlap
  (params (OtherActor :type Actor%20Object%20Reference))
  (bind _returnvalue (Transformation|GetActorLocation))
  (bind _fx2 (Variables|Default|Getfx2))
  ;[0.04971 0.04971 0.04971] Target Spell detracts from structure strength and destroys on 5th hit
  (Utilities|Casting|CastToBP_TargetSpell OtherActor)
  (Variables|Default|SetStructure (- (Variables|Default|GetStructure) 1.0))
  (Transformation|SetRelativeTransform _fx2 (Math|Transform|MakeTransform "0, 0, 0" "0, 0, 0" (- (Variables|/Script/Engine.SceneComponent|GetRelativeScale3D _fx2) "0.025000,0.025000,0.009590")) false false)
  (if (<= (Variables|Default|GetStructure) 0.0)
    (Effects|SpawnEmitteratLocation "/Game/VisualEffects/FXVarietyPack/Particles/P_ky_lightning2.P_ky_lightning2" _returnvalue "0, 0, 0" "4.000000,4.000000,4.000000")
    (Utilities|FlowControl|Delay 1.0)
    (Actor|DestroyActor)
    (Effects|SpawnEmitteratLocation "/Game/VisualEffects/RealisticVFX/Particles/Environment/P_Butterfly.P_Butterfly" _returnvalue)))

(fn ConstructionScript)