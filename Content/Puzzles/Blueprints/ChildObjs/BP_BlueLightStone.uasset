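; BP_BlueLightStone is a puzzle stone, built as a child Blueprint, that snaps into place when it reaches a rock detector.
; When BoxOverlap begins overlapping a BP_RockDetector, it moves the Box, MagnetMesh and BoxOverlap components to the detector's root location.
; It then turns off physics simulation on MagnetMesh so the stone stays put.
; The construction script only calls the parent's.
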(event OnComponentBeginOverlap(BoxOverlap)
  (params (OverlappedComponent :type Primitive%20Component%20Object%20Reference) (OtherActor :type Actor%20Object%20Reference) (OtherComp :type Primitive%20Component%20Object%20Reference) (OtherBodyIndex :type Integer) (bFromSweep :type Boolean) (SweepResult :type Hit%20Result%20Structure%20%28by%20ref%29))
  ;[0.04971 0.04971 0.04971] Positioning Rock Upon Drop Obj (RockDectector)
  (bind _asbp_rock_detector (Utilities|Casting|CastToBP_RockDetector OtherActor))
  (if (== OtherActor _asbp_rock_detector)
    (bind _output_get (Variables|Default|SetRockLocation (Transformation|GetWorldLocation (Variables|/Script/Engine.Actor|GetRootComponent _asbp_rock_detector))))
    (Transformation|SetWorldLocation (Variables|Default|GetBox) (+ _output_get "") false false)
    (Physics|SetSimulatePhysics (Variables|Default|GetMagnetMesh) false)))

(fn ConstructionScript
  (|CallParentFunction))