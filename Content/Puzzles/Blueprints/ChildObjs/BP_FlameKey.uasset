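; BP_FlameKey is a puzzle key that raises a flame in stages to remove the Level 3 shield barrier.
; FlameCount increments a counter: one starts the FlameRise timeline, gated by SingleFlame, and two plays FinalFlame if both OnlyPyramid flags are set.
; Both timelines move FlameHolder and Capsule, spawning hit particles every update.
; FinalFlame updates also call FlameShieldChange, which spawns effects at checkpoint 3 and destroys the barriers after a delay.
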(event Custom|FlameKey
  ;[0.04971 0.04971 0.04971] FinalFlame Animation & Position Transform on FlameCount = 2
  (if (== (Variables|Default|GetFlameCounter) 2)
    (if (Variables|Default|GetOnlyPyramid1)
      (if (Variables|Default|GetOnlyPyramid2)
        (bind _finalflame (Timeline|FinalFlame Play)
          (:Update
            (Transformation|SetRelativeLocation (Variables|Default|GetFlameHolder) _finalflame false false)
            (Effects|SpawnEmitteratLocation "/Game/VisualEffects/FXVarietyPack/Particles/P_ky_hit2.P_ky_hit2" (Transformation|GetActorLocation) "0, 0, 0" "2.300000,2.300000,2.300000")
            (CallFunction|FlameShieldChange)))))))

(event Custom|FlameShieldChange
  (bind _location (Variables|Default|GetLocation))
  ;[0.04971 0.04971 0.04971] Hide Barrier
  (Effects|SpawnEmitteratLocation "/Game/VisualEffects/RealisticVFX/Particles/Destruction/P_Destruction_Electric.P_Destruction_Electric" _location "0, 0, 0" "1.800000,1.800000,1.800000")
  (Utilities|FlowControl|Delay 5.5)
  (bind _outactors (Actor|GetAllActorsOfClass "/Game/Puzzles/Blueprints/ChildObjs/BP_Level3ShieldBarrier.BP_Level3ShieldBarrier_C"))
  (Actor|DestroyActor _outactors)
  (Effects|SpawnEmitteratLocation "/Game/VisualEffects/RealisticVFX/Particles/Environment/P_Butterfly.P_Butterfly" _location))

(event Custom|StartFlame
  ;[0.04971 0.04971 0.04971] Starting Flame Animation When SingleFlame Is Detected
  (if (Variables|Default|GetSingleFlame)
    (bind _flamerise (Timeline|FlameRise Play)
      (:Update
        (Transformation|SetRelativeLocation (Variables|Default|GetFlameHolder) _flamerise false false)
        (Effects|SpawnEmitteratLocation "/Game/VisualEffects/FXVarietyPack/Particles/P_ky_hit2.P_ky_hit2" (Transformation|GetActorLocation) "0, 0, 0" "2.300000,2.300000,2.300000")
        (Variables|Default|SetSingleFlame false)))))

(event Custom|FlameCount
  ;[0.04971 0.04971 0.04971] Incrementing FlameCounter, Initialising SingleFlame & Executing Function
  (if (<= (Variables|Default|GetFlameCounter) 1)
    (Variables|Default|SetFlameCounter (+ (Variables|Default|GetFlameCounter) (Variables|Default|GetCount)))
    (if (== (Variables|Default|GetFlameCounter) 1) :!label _label
      (CallFunction|StartFlame)
      (elif (== (Variables|Default|GetFlameCounter) 2)
        (CallFunction|FlameKey)
        (else
          (goto _label))))))

(event EventBeginPlay
  ;[0.04971 0.04971 0.04971] Setting Location On EventBeginPlay
  (Actor|GetActorOfClass "/Game/Puzzles/Blueprints/ChildObjs/BP_Level3ShieldBarrier.BP_Level3ShieldBarrier_C")
  (bind _returnvalue (Actor|GetActorOfClass "/Game/ThirdPerson/Blueprints/RespawnCheckpoints/BP_RespawnCheckpoint3.BP_RespawnCheckpoint3_C"))
  (Variables|Default|SetLocation (Transformation|GetActorLocation _returnvalue)))

(fn ConstructionScript)