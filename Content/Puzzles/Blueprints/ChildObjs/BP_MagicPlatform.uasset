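; BP_MagicPlatform is a puzzle object that flags itself as a magic platform and reports flame progress to BP_FlameKey.
; When its capsule is overlapped while MagicItem is set, it finds the key actor and flags which of two pyramids it belongs to.
; It then pulses SingleFlame around a FlameCount call and clears MagicItem, so each set of that flag counts once.
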(event OnComponentBeginOverlap(Capsule)
  (params (OverlappedComponent :type Primitive%20Component%20Object%20Reference) (OtherActor :type Actor%20Object%20Reference) (OtherComp :type Primitive%20Component%20Object%20Reference) (OtherBodyIndex :type Integer) (bFromSweep :type Boolean) (SweepResult :type Hit%20Result%20Structure%20%28by%20ref%29))
  ;[0.04971 0.04971 0.04971] Checking for MagicItem Upon Collision Overlap
  (if (Variables|Default|GetMagicItem)
    (bind _returnvalue (Actor|GetActorOfClass "/Game/Puzzles/Blueprints/ChildObjs/BP_FlameKey.BP_FlameKey_C"))
    (if (Variables|Default|GetMagicPyramid1)
      (Variables|/Game/Puzzles/Blueprints/ChildObjs/BP_FlameKey.BP_FlameKey_C|SetOnlyPyramid1 _returnvalue true)
      (Variables|/Game/Puzzles/Blueprints/ChildObjs/BP_FlameKey.BP_FlameKey_C|SetSingleFlame _returnvalue true :!label _label)
      (Default|FlameCount _returnvalue)
      (Variables|Default|SetMagicItem false)
      (Variables|/Game/Puzzles/Blueprints/ChildObjs/BP_FlameKey.BP_FlameKey_C|SetSingleFlame _returnvalue false)
      (elif (Variables|Default|GetMagicPyramid2)
        (Variables|/Game/Puzzles/Blueprints/ChildObjs/BP_FlameKey.BP_FlameKey_C|SetOnlyPyramid2 _returnvalue true)
        (goto _label)))))

(event EventBeginPlay
  ;[0.04971 0.04971 0.04971] Setting Counter & MagicRope on Begin Play
  (Variables|Default|SetMagicPlatform true)
  (Variables|Default|SetMagicItem false))

(fn ConstructionScript)