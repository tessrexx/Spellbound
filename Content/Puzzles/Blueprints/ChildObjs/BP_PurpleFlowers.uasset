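; Purple flowers puzzle object that opens the fire barrier when placed on its BP_PurpleStand.
; When its overlap box touches the stand, it moves its mesh and boxes to just above the stand and disables the mesh's physics.
; It then calls DestroyFireBarrier, which destroys every BP_RedBarrier in the level through a class-wide actor search rather than a specific reference.
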(event OnComponentBeginOverlap(BoxOverlap)
  (params (OverlappedComponent :type Primitive%20Component%20Object%20Reference) (OtherActor :type Actor%20Object%20Reference) (OtherComp :type Primitive%20Component%20Object%20Reference) (OtherBodyIndex :type Integer) (bFromSweep :type Boolean) (SweepResult :type Hit%20Result%20Structure%20%28by%20ref%29))
  (bind _magnetmesh (Variables|Default|GetMagnetMesh))
  ;[0.04971 0.04971 0.04971] Positioning Flowers Upon Drop Obj (PurpleStand)
  (bind _aspurple_stand (Utilities|Casting|CastToBP_PurpleStand OtherActor))
  (if (== OtherActor _aspurple_stand)
    (bind _output_get (Variables|Default|SetFlowerLocation (Transformation|GetWorldLocation (Variables|/Script/Engine.Actor|GetRootComponent _aspurple_stand))))
    (Transformation|SetWorldLocation _magnetmesh (+ _output_get "0,0,50.000000") false false)
    (Physics|SetSimulatePhysics _magnetmesh false)
    ;[0.04971 0.04971 0.04971] Call Destroy Barrier Function
    (CallFunction|DestroyFireBarrier)))

(event Custom|DestroyFireBarrier
  ;[0.04971 0.04971 0.04971] Destroy FireBarrier
  (bind _outactors (Actor|GetAllActorsOfClass "/Game/Puzzles/Blueprints/ChildObjs/BP_RedBarrier.BP_RedBarrier_C"))
  (Actor|DestroyActor _outactors))

(fn ConstructionScript)