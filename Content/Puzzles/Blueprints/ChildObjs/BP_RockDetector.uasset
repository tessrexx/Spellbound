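; BP_RockDetector is a puzzle trigger that removes the blue barrier when a BlueLightStone overlaps its box collider.
; On a valid overlap, it finds a BP_BlueBarrier by class, spawns hit and butterfly particles at its location, then destroys it after a short delay.
; BeginPlay also stores the button's resting and lowered relative transforms, but nothing in these graphs moves the button.
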(event OnComponentBeginOverlap(BoxCollider)
  (params (OverlappedComponent :type Primitive%20Component%20Object%20Reference) (OtherActor :type Actor%20Object%20Reference) (OtherComp :type Primitive%20Component%20Object%20Reference) (OtherBodyIndex :type Integer) (bFromSweep :type Boolean) (SweepResult :type Hit%20Result%20Structure%20%28by%20ref%29))
  ;[0.04971 0.04971 0.04971] Destroying BP_BlueBarrier upon collision
  (bind _asblue_light_stone (Utilities|Casting|CastToBlueLightStone OtherActor))
  (if (Variables|/Game/Puzzles/Blueprints/ChildObjs/BlueLightStone.BlueLightStone_C|GetBlueLightStone _asblue_light_stone)
    (bind _returnvalue (Actor|GetActorOfClass "/Game/Puzzles/Blueprints/ChildObjs/BP_BlueBarrier.BP_BlueBarrier_C"))
    ;;[0 0 0] EmitterAnimations Collapse
    (|EmitterAnimations _returnvalue)
    (Utilities|FlowControl|Delay 0.3)
    (Actor|DestroyActor _returnvalue)))

(event EventBeginPlay
  (bind _button (Variables|Default|GetButton))
  (bind _returnvalue (Transformation|GetRelativeTransform _button))
  ;[0.04971 0.04971 0.04971] Setting Relative Location On EventBeginPlay
  (Variables|Default|SetStart (Math|Transform|MakeTransform (.location _returnvalue) (.rotation _returnvalue) (.scale _returnvalue)))
  (Variables|Default|SetEnd (Math|Transform|MakeTransform (- (.location _returnvalue) "0,0,10.000000") (.rotation _returnvalue) (.scale _returnvalue))))

(fn ConstructionScript)