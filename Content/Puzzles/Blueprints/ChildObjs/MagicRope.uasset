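; MagicRope is a puzzle object that reacts when a MagicLantern overlaps its capsule, with only debug counting implemented so far.
; BeginPlay sets Count to one and prints it.
; On overlap, if the lantern's MagicLanternTall flag is set, it copies Count into Counter by adding zero and prints it, so nothing increments.
; An unconnected cast to MagicLamp never runs.
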(event OnComponentBeginOverlap(Capsule)
  (params (OverlappedComponent :type Primitive%20Component%20Object%20Reference) (OtherActor :type Actor%20Object%20Reference) (OtherComp :type Primitive%20Component%20Object%20Reference) (OtherBodyIndex :type Integer) (bFromSweep :type Boolean) (SweepResult :type Hit%20Result%20Structure%20%28by%20ref%29))
  (bind _asmagic_lantern (Utilities|Casting|CastToMagicLantern OtherActor))
  (if (Variables|/Game/Puzzles/Blueprints/ChildObjs/MagicLantern.MagicLantern_C|GetMagicLanternTall _asmagic_lantern)
    (bind _output_get (Variables|Default|SetCounter (+ (Variables|Default|GetCount) 0)))
    (Development|PrintString "Counter =")
    (Development|PrintString (Utilities|String|ToString(Integer) _output_get))))

(event EventBeginPlay
  (bind _output_get (Variables|Default|SetCount 1))
  (Development|PrintString "Count Set")
  (Development|PrintString (Utilities|String|ToString(Integer) _output_get)))

(fn ConstructionScript)