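; PurpleFlowers is a puzzle object, the purple flowers that snap onto a PurpleStand when dropped.
; On BeginPlay it sets its PurpleFlowers flag, which a comment says triggers functionality within MagicStatue.
; Any BoxOverlap begin overlap, with no filter on the other actor, looks up the PurpleStand by class and moves MagnetMesh, Box and BoxOverlap just above it.
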(event OnComponentBeginOverlap(BoxOverlap)
  (params (OverlappedComponent :type Primitive%20Component%20Object%20Reference) (OtherActor :type Actor%20Object%20Reference) (OtherComp :type Primitive%20Component%20Object%20Reference) (OtherBodyIndex :type Integer) (bFromSweep :type Boolean) (SweepResult :type Hit%20Result%20Structure%20%28by%20ref%29))
  ;[0.04971 0.04971 0.04971] Positioning Flowers Upon Drop Obj
  (bind _returnvalue (Actor|GetActorOfClass "/Game/Puzzles/Blueprints/ChildObjs/PurpleStand.PurpleStand_C"))
  (bind _output_get (Variables|Default|SetFlowerLocation (Transformation|GetWorldLocation (Variables|/Script/Engine.Actor|GetRootComponent _returnvalue))))
  (Transformation|SetWorldLocation (Variables|Default|GetMagnetMesh) (+ _output_get "0,0,50.000000") false false))

(event EventBeginPlay
  ;[0.04971 0.04971 0.04971] Setting PurpleFlowers to True: Triggers functionality within MagicStatue
  (Variables|Default|SetPurpleFlowers true))

(fn ConstructionScript)