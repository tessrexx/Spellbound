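; PurpleStand is a puzzle stand Blueprint that reports to a MagicStatue when something overlaps its sphere while ButtonPressed is true.
; On overlap it finds the first MagicStatue in the level, sets that statue's Button1 flag and calls its MagicStatue event.
; Debug prints trace each step, and nothing in this graph sets ButtonPressed.
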(event OnComponentBeginOverlap(Sphere)
  (params (OverlappedComponent :type Primitive%20Component%20Object%20Reference) (OtherActor :type Actor%20Object%20Reference) (OtherComp :type Primitive%20Component%20Object%20Reference) (OtherBodyIndex :type Integer) (bFromSweep :type Boolean) (SweepResult :type Hit%20Result%20Structure%20%28by%20ref%29))
  (Development|PrintString "BeginOverlap")
  (if (Variables|Default|GetButtonPressed)
    (Development|PrintString "ButtonPressed True")
    (bind _outactors (Actor|GetAllActorsOfClass "/Game/Puzzles/Blueprints/MagicStatue.MagicStatue_C"))
    (bind _output_get (Variables|Default|SetStatRef (Utilities|Array|Get(acopy) _outactors)))
    (Development|PrintString "StatRefSet")
    (Variables|/Game/Puzzles/Blueprints/MagicStatue.MagicStatue_C|SetButton1 _output_get true)
    (Default|MagicStatue _output_get)
    (Development|PrintString "MagicStatueExec")))

(fn ConstructionScript)