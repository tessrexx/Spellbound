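; FlameKey is a puzzle key whose flame rises in two stages, the second hiding the Level3ShieldBarrier.
; FlameCount increments a counter, triggering the FlameRise timeline at one (gated by SingleFlame) and FinalFlame at two.
; Both timelines move the FlameHolder and Capsule, spawning particles on every update.
; FinalFlame's updates also call FlameShieldChange, which spawns electric destruction at the barrier's cached location, then hides it after a delay.
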(event Custom|FlameKey
  (bind _returnvalue (Transformation|GetActorLocation))
  ;[0.04971 0.04971 0.04971] FinalFlame Animation & Position Transform on FlameCount = 2
  (if (== (Variables|Default|GetFlameCounter) 2)
    (Development|PrintString "Huge Flame")
    (bind _finalflame (Timeline|FinalFlame Play)
      (:Update
        (Transformation|SetRelativeLocation (Variables|Default|GetFlameHolder) _finalflame false false)
        (Effects|SpawnEmitteratLocation "/Game/VisualEffects/FXVarietyPack/Particles/P_ky_hit2.P_ky_hit2" _returnvalue "0, 0, 0" "2.300000,2.300000,2.300000")
        (Effects|SpawnEmitteratLocation "/Game/VisualEffects/RealisticVFX/Particles/Environment/P_Butterfly.P_Butterfly" _returnvalue)
        (CallFunction|FlameShieldChange)))))

(event Custom|FlameShieldChange
  (Effects|SpawnEmitteratLocation "/Game/VisualEffects/RealisticVFX/Particles/Destruction/P_Destruction_Electric.P_Destruction_Electric" (Variables|Default|GetLocation) "0, 0, 0" "2.300000,2.300000,2.300000")
  (Utilities|FlowControl|Delay 2.3)
  (bind _returnvalue (Actor|GetActorOfClass "/Game/Puzzles/Blueprints/ChildObjs/Level3ShieldBarrier.Level3ShieldBarrier_C"))
  (Rendering|SetActorHiddenInGame _returnvalue true))

(event Custom|StartFlame
  ;[0.04971 0.04971 0.04971] Starting Flame Animation When SingleFlame Is Detected
  (if (Variables|Default|GetSingleFlame)
    (Development|PrintString "FlameStarted")
    (bind _flamerise (Timeline|FlameRise Play)
      (:Update
        (Transformation|SetRelativeLocation (Variables|Default|GetFlameHolder) _flamerise false false)
        (Effects|SpawnEmitteratLocation "/Game/VisualEffects/FXVarietyPack/Particles/P_ky_hit2.P_ky_hit2" (Transformation|GetActorLocation) "0, 0, 0" "2.300000,2.300000,2.300000")
        (Variables|Default|SetSingleFlame false)))))

(event Custom|FlameCount
  ;[0.04971 0.04971 0.04971] Incrementing FlameCounter, Initialising SingleFlame & Executing Function
  (if (<= (Variables|Default|GetFlameCounter) 1)
    (bind _output_get (Variables|Default|SetFlameCounter (+ (Variables|Default|GetFlameCounter) (Variables|Default|GetCount))))
    (Development|PrintString "Counter =")
    (Development|PrintString (Utilities|String|ToString(Integer) _output_get))
    (if (== (Variables|Default|GetFlameCounter) 1) :!label _label
      (CallFunction|StartFlame)
      (elif (== (Variables|Default|GetFlameCounter) 2)
        (CallFunction|FlameKey)
        (else
          (goto _label))))))

(event EventBeginPlay
  ;[0.04971 0.04971 0.04971] Setting Location On EventBeginPlay
  (bind _returnvalue (Actor|GetActorOfClass "/Game/Puzzles/Blueprints/ChildObjs/Level3ShieldBarrier.Level3ShieldBarrier_C"))
  (Variables|Default|SetLocation (Transformation|GetActorLocation _returnvalue)))

(fn ConstructionScript)