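; Parent puzzle button for drop-object interactions, pressed with the DropItemInteract input while something overlaps its capsule.
; BeginPlay caches the button's out and pressed-in transforms and enables player input, and capsule overlaps open and close a Gate that filters that input.
; A press plays a sound, lerps the button in and back out through two timelines, and sets ButtonPressed from the return animation's update; no drop logic lives here.
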(event OnComponentBeginOverlap(CapsuleCollider)
  (params (OverlappedComponent :type Primitive%20Component%20Object%20Reference) (OtherActor :type Actor%20Object%20Reference) (OtherComp :type Primitive%20Component%20Object%20Reference) (OtherBodyIndex :type Integer) (bFromSweep :type Boolean) (SweepResult :type Hit%20Result%20Structure%20%28by%20ref%29))
  ;[0.04971 0.04971 0.04971] Button Interation
  (Utilities|FlowControl|Gate true) ; enters at Open
)

(event OnComponentEndOverlap(CapsuleCollider)
  (params (OverlappedComponent :type Primitive%20Component%20Object%20Reference) (OtherActor :type Actor%20Object%20Reference) (OtherComp :type Primitive%20Component%20Object%20Reference) (OtherBodyIndex :type Integer))
  ;[0.04971 0.04971 0.04971] Button Interation
  (Utilities|FlowControl|Gate true) ; enters at Close
)

(event EventBeginPlay
  (bind _button (Variables|Default|GetButton))
  (bind _returnvalue (Transformation|GetRelativeTransform _button))
  ;[0.04971 0.04971 0.04971] Set Button Input, Output & Enable Player Control
  (Variables|Default|SetOutPosition (Math|Transform|MakeTransform (.location _returnvalue) (.rotation _returnvalue) (.scale _returnvalue)))
  (Variables|Default|SetInPosition (Math|Transform|MakeTransform (- (.location _returnvalue) "0,0,10.000000") (.rotation _returnvalue) (.scale _returnvalue)))
  (Input|EnableInput (Game|GetPlayerController 0)))

(event Input|ActionEvents|InputActionDropItemInteract
  (params (Key :type Key%20Structure :default "None"))
  ;[0.04971 0.04971 0.04971] Button Interation
  (:Pressed
    (Utilities|FlowControl|Gate true
      (:Exit
        ;[0.04971 0.04971 0.04971] Button Animations
        (|ButtonAnimations
          (:Out
            ;[0.04971 0.04971 0.04971] Setting ButtonPressed To True
            (Variables|Default|SetButtonPressed true)))))))

(fn ConstructionScript)