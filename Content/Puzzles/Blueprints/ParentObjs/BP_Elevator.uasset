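; Puzzle elevator Blueprint that moves the elevator mesh and its trigger box up or down along timelines.
; Overlapping the box plays ElevatorAnimation until the sphere is touched, which sets a pickup flag that is never reset.
; With the flag set, either overlap plays ElevatorDown after a short delay.
; The ElevatorPickup component destroys itself when an overlap with it ends.
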(event OnComponentEndOverlap(ElevatorPickup)
  (params (OverlappedComponent :type Primitive%20Component%20Object%20Reference) (OtherActor :type Actor%20Object%20Reference) (OtherComp :type Primitive%20Component%20Object%20Reference) (OtherBodyIndex :type Integer))
  ;[0.04971 0.04971 0.04971] Destroy Elevator Pickup
  (Components|DestroyComponent (Variables|Default|GetElevatorPickup)))

(event OnComponentBeginOverlap(Box)
  (params (OverlappedComponent :type Primitive%20Component%20Object%20Reference) (OtherActor :type Actor%20Object%20Reference) (OtherComp :type Primitive%20Component%20Object%20Reference) (OtherBodyIndex :type Integer) (bFromSweep :type Boolean) (SweepResult :type Hit%20Result%20Structure%20%28by%20ref%29))
  ;[0.04971 0.04971 0.04971] Elevator Up/Down
  (if (Variables|Default|GetIsPickupTouched)
    (Utilities|FlowControl|Delay 2.23)
    (bind _moveelevator (Timeline|ElevatorDown Play)
      (:Update
        (Transformation|SetRelativeLocation (Variables|Default|GetElevatorMesh) _moveelevator false false)))
    (else
      (bind _moveelevator_2 (Timeline|ElevatorAnimation Play)
        (:Update
          (Transformation|SetRelativeLocation (Variables|Default|GetElevatorMesh) _moveelevator_2 false false))))))

(event OnComponentBeginOverlap(Sphere)
  (params (OverlappedComponent :type Primitive%20Component%20Object%20Reference) (OtherActor :type Actor%20Object%20Reference) (OtherComp :type Primitive%20Component%20Object%20Reference) (OtherBodyIndex :type Integer) (bFromSweep :type Boolean) (SweepResult :type Hit%20Result%20Structure%20%28by%20ref%29))
  ;[0.04971 0.04971 0.04971] Elevator Up/Down
  (Variables|Default|SetIsPickupTouched true)
  (if (Variables|Default|GetIsPickupTouched)
    (Utilities|FlowControl|Delay 2.23)
    (bind _moveelevator (Timeline|ElevatorDown Play)
      (:Update
        (Transformation|SetRelativeLocation (Variables|Default|GetElevatorMesh) _moveelevator false false)))
    (else
      (bind _moveelevator_2 (Timeline|ElevatorAnimation Play)
        (:Update
          (Transformation|SetRelativeLocation (Variables|Default|GetElevatorMesh) _moveelevator_2 false false))))))

(fn ConstructionScript)