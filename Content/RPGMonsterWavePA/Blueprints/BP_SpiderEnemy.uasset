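; BP_SpiderEnemy is a spider enemy Blueprint that handles taking damage and dying.
; Each AnyDamage event removes one health point regardless of damage amount, plays a hurt montage and waits for its length.
; When health is depleted, it plays a death montage, spawns a hit particle after a short delay, stops the AI controller's brain logic and destroys the actor.
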(event Game|Damage|EventAnyDamage
  (params (Damage :type Float%20%28single-precision%29) (DamageType :type Damage%20Type%20Object%20Reference) (InstigatedBy :type Controller%20Object%20Reference) (DamageCauser :type Actor%20Object%20Reference))
  ;[0.04971 0.04971 0.04971] Enemy Takes Damage (reduces health and death)
  (bind _output_get (Variables|Default|SetSpiderHealth (- (Variables|Default|GetSpiderHealth) 1)))
  (bind _returnvalue (Animation|PlayAnimMontage "/Game/RPGMonsterWavePA/EnemyAnimation/SpiderHurtMontage.SpiderHurtMontage" 1.0 "None"))
  (Utilities|FlowControl|Delay _returnvalue)
  (if (<= _output_get 0)
    (Animation|PlayAnimMontage "/Game/RPGMonsterWavePA/EnemyAnimation/SpiderDeathMontage.SpiderDeathMontage" 1.0 "None")
    (Utilities|FlowControl|Delay 0.75)
    (Effects|SpawnEmitteratLocation "/Game/VisualEffects/FXVarietyPack/Particles/P_ky_hit1.P_ky_hit1" (Transformation|GetActorLocation))
    (AI|Logic|StopLogic (Variables|/Script/AIModule.AIController|GetBrainComponent (AI|GetAIController self)) "")
    (Actor|DestroyActor)))

(fn ConstructionScript)